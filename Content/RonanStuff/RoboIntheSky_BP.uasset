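; RoboIntheSky_BP is an actor, likely a flying robot going by its name, that moves along a short path using an InterpToMovement component.
; The construction script builds the path from relative control points: the origin, then the Position1 and Position2 variables.
; It also passes the Duration variable in as the interpolation time.
; The event graph holds only disabled default events, so the Blueprint adds no runtime logic.
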(event EventBeginPlay
  (|CallParentFunction) ; This node is disabled and will not be called.\nDrag off pins to build functionality.
)

(event Collision|EventActorBeginOverlap
  (params (OtherActor :type Actor%20Object%20Reference))
  (|CallParentFunction OtherActor) ; This node is disabled and will not be called.\nDrag off pins to build functionality.
)

(event EventTick
  (params (DeltaSeconds :type Float%20%28single-precision%29))
  (|CallParentFunction DeltaSeconds) ; This node is disabled and will not be called.\nDrag off pins to build functionality.
)

(fn ConstructionScript
  (bind _interptomovement (Variables|Default|GetInterpToMovement))
  (|CallParentFunction)
  (Class|InterptoMovementComponent|AddControlPointPosition _interptomovement "0, 0, 0" true)
  (Class|InterptoMovementComponent|AddControlPointPosition _interptomovement (Variables|Default|GetPosition1) true)
  (Class|InterptoMovementComponent|AddControlPointPosition _interptomovement (Variables|Default|GetPosition2) true)
  (Class|SubmixEffectDelayStatics|SetInterpolationTime (Utilities|Struct|MakeSubmixEffectDelaySettings 2e+03 4e+02 1e+03) (Variables|Default|GetDuration)))