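; Box_BP is a construction-time placement tool that adds instances of the Box mesh component along configurable lines.
; Three nested loops in the construction script use Length, LengthY and LengthZ, each with its own per-axis spacing.
; Each instance's location depends only on its own loop index, so inner loops restack identical lines on each outer pass instead of forming a grid.
; The event graph holds no active logic.
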(event EventBeginPlay)

(event Collision|EventActorBeginOverlap
  (params (OtherActor :type Actor%20Object%20Reference)))

(event EventTick
  (params (DeltaSeconds :type Float%20%28single-precision%29)))

(fn ConstructionScript
  (for _index (range 0 (Variables|Default|GetLength))
    (Components|InstancedStaticMesh|AddInstance (Variables|Default|GetBox) (Math|Transform|MakeTransform (Math|Vector|MakeVector (* _index (Variables|Default|GetDistanceX)) (* _index (Variables|Default|GetDistanceY)) (* _index (Variables|Default|GetDistanceZ))) "0, 0, 0" "1.000000,1.000000,1.000000") false)
    (for _index_2 (range 0 (Variables|Default|GetLengthY))
      (Components|InstancedStaticMesh|AddInstance (Variables|Default|GetBox) (Math|Transform|MakeTransform (Math|Vector|MakeVector (* _index_2 (Variables|Default|GetDistanceX2)) (* _index_2 (Variables|Default|GetDistanceY2)) (* _index_2 (Variables|Default|GetDistanceZ2))) "0, 0, 0" "1.000000,1.000000,1.000000") false)
      (for _index_3 (range 0 (Variables|Default|GetLengthZ))
        (Components|InstancedStaticMesh|AddInstance (Variables|Default|GetBox) (Math|Transform|MakeTransform (Math|Vector|MakeVector (* _index_3 (Variables|Default|GetDistanceX3)) (* _index_3 (Variables|Default|GetDistanceY3)) (* _index_3 (Variables|Default|GetDistanceZ3))) "0, 0, 0" "1.000000,1.000000,1.000000") false)))))