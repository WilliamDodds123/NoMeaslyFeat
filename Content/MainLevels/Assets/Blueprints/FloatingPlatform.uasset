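; Floating platform Blueprint that shuttles its static mesh back and forth between two points of its spline in an endless loop.
; Two chained MoveComponentTo calls target local-space locations at variable-selected point indices, so the spline only supplies endpoints rather than a path to follow.
; The first leg's duration comes from the Time variable, while the second is fixed.
; A Repeat custom event restarts the sequence begun on BeginPlay.
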(event Custom|Repeat
  (Components|MoveComponentTo (Variables|Default|GetStaticMesh) (Spline|GetLocationatSplinePoint (Variables|Default|GetSpline) (Variables|Default|GetSplinePointsNum) "Local") "0, 0, 0" false false (Variables|Default|GetTime) false)
  (Components|MoveComponentTo (Variables|Default|GetStaticMesh) (Spline|GetLocationatSplinePoint (Variables|Default|GetSpline) (Variables|Default|GetSpline%20Num%202) "Local") "0, 0, 0" false false 5.0 false)
  (CallFunction|Repeat))

(event EventBeginPlay
  (Components|MoveComponentTo (Variables|Default|GetStaticMesh) (Spline|GetLocationatSplinePoint (Variables|Default|GetSpline) (Variables|Default|GetSplinePointsNum) "Local") "0, 0, 0" false false (Variables|Default|GetTime) false)
  (Components|MoveComponentTo (Variables|Default|GetStaticMesh) (Spline|GetLocationatSplinePoint (Variables|Default|GetSpline) (Variables|Default|GetSpline%20Num%202) "Local") "0, 0, 0" false false 5.0 false)
  (CallFunction|Repeat))

(fn ConstructionScript)