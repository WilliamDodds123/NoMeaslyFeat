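; Spawner actor that drops crates for the conveyor belt.
; BeginPlay caches the StartDropCrate actor, whose StartDroppingBlocks flag gates spawning.
; Tick feeds a Delay that acts as a repeating timer of about three seconds, then checks that flag.
; When it is set, a CrateBP spawns at the world transform of one of four randomly picked Arrow components, ignoring collision.
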(event EventBeginPlay
  (bind _returnvalue (Actor|GetActorOfClass "/Game/MainLevels/Assets/Blueprints/ConveyorBelt/StartDropCrate.StartDropCrate_C")))

(event EventTick
  (params (DeltaSeconds :type Float%20%28single-precision%29))
  (Utilities|FlowControl|Delay 3.0)
  (if (Variables|/Game/MainLevels/Assets/Blueprints/ConveyorBelt/StartDropCrate.StartDropCrate_C|GetStartDroppingBlocks (stale EventBeginPlay _returnvalue))
    (Game|SpawnActorfromClass "/Game/MainLevels/Assets/Blueprints/ConveyorBelt/CrateBP.CrateBP_C" (Transformation|GetWorldTransform (.OutItem (Utilities|Array|Random (Utilities|Array|MakeArray (Variables|Default|GetArrow) (Variables|Default|GetArrow1) (Variables|Default|GetArrow2) (Variables|Default|GetArrow3))))) "AlwaysSpawn" 0 0)))

(fn ConstructionScript)