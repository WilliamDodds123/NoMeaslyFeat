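; LightWall_BP is a modular wall actor that builds a straight row of wall and cover pieces in the construction script.
; A loop over Number fills two transform arrays at 100-unit steps along local X, which are batch-added to the Wall and WallCover instanced mesh components.
; The event graph holds only disabled placeholder events, so it adds no runtime logic.
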(event EventBeginPlay)

(event Collision|EventActorBeginOverlap
  (params (OtherActor :type Actor%20Object%20Reference)))

(event EventTick
  (params (DeltaSeconds :type Float%20%28single-precision%29)))

(fn ConstructionScript
  (for _index (range 0 (- (Variables|Default|GetNumber) 1))
    (Utilities|Array|Add (Variables|Default|GetWall%20Cover%20Transforms) (Math|Transform|MakeTransform (Math|Vector|MakeVector (* _index 1e+02) 0.0 0.0)))
    (Utilities|Array|Add (Variables|Default|GetWall%20Transforms) (Math|Transform|MakeTransform (Math|Vector|MakeVector (* _index 1e+02) 0.0 0.0))))
  (Components|InstancedStaticMesh|AddInstances (Variables|Default|GetWall) (Variables|Default|GetWall%20Transforms) false false)
  (Components|InstancedStaticMesh|AddInstances (Variables|Default|GetWallCover) (Variables|Default|GetWall%20Cover%20Transforms) false false))